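; Player-controlled basket for an apple-picking game that visually fills up with caught apples.
; MoveAxisX and MoveAxisY share one world-offset move scaled by Speed and delta time, while Tick applies any pending movement input as a swept local offset.
; On overlap, the basket copies the other component's static mesh into the next ApplesArray slot, clearing all slots and the counter once full.
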(event `self.ReceiveTick`
  (params (DeltaSeconds :type "Float (single-precision)"))
  (bind _returnvalue (`self.ConsumeMovementInputVector`))
  (`self.K2_AddActorLocalOffset` (* _returnvalue DeltaSeconds) true))

(event `InputAxis|MoveAxisX`
  (params (AxisValue :type "Float (single-precision)"))
  (bind _returnvalue (`GameplayStatics.GetWorldDeltaSeconds`))
  (bind _speed (`self.Speed`))
  (`self.K2_AddActorWorldOffset` (`KismetMathLibrary.MakeVector` (* AxisValue _speed _returnvalue) (* (stale `InputAxis|MoveAxisY` AxisValue) _speed _returnvalue)) :!label _label))

(event `InputAxis|MoveAxisY`
  (params (AxisValue :type "Float (single-precision)"))
  (goto _label))

(event `self.SM_Basket.OnComponentBeginOverlap`
  (params (OverlappedComponent :type "PrimitiveComponent Object Reference") (OtherActor :type "Actor Object Reference") (OtherComp :type "PrimitiveComponent Object Reference") (OtherBodyIndex :type Integer) (bFromSweep :type Boolean) (SweepResult :type "HitResult Structure (by ref)"))
  (bind _countharvestapple (`self.CountHarvestApple`))
  (bind _array (`|MakeArray` (`self.SM_Apple0`) (`self.SM_Apple1`) (`self.SM_Apple2`) (`self.SM_Apple3`) (`self.SM_Apple4`) (`self.SM_Apple5`) (`self.SM_Apple6`) (`self.SM_Apple7`) (`self.SM_Apple8`) (`self.SM_Apple9`) (`self.SM_Apple10`) (`self.SM_Apple11`) (`self.SM_Apple12`) (`self.SM_Apple13`) (`self.SM_Apple14`) (`self.SM_Apple15`) (`self.SM_Apple16`) (`self.SM_Apple17`) (`self.SM_Apple18`) (`self.SM_Apple19`) (`self.SM_Apple20`) (`self.SM_Apple21`) (`self.SM_Apple22`)))
  (bind _returnvalue (`KismetArrayLibrary.Array_Length` _array))
  ;[1 1 1] Get overlapped static mesh
  (bind _asstatic_mesh_component (cast `StaticMeshComponent` OtherComp))
  (`StaticMeshComponent.SetStaticMesh` (`|GetArrayItem` _array (`self.CountHarvestApple`)) (`StaticMeshComponent.StaticMesh` _asstatic_mesh_component))
  (`/Engine/EditorBlueprintResources/StandardMacros.IncrementInt` _countharvestapple
    (:`  `
      ;[1 1 1] Reset static mash apples if the basket is full
      (if (not (< _countharvestapple _returnvalue))
        (for _index (range (+ _returnvalue 1))
          (`StaticMeshComponent.SetStaticMesh` (`|GetArrayItem` _array _index) null)
          (set `self.CountHarvestApple` 0))))))

(fn `UserConstructionScript`)