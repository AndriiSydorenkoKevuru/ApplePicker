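; BP_AppleTree is a tree actor that drops a burst of apples when a BP_Basket hits its static mesh.
; A hit distance check, meant to take only the first hit, starts a custom delayed-loop macro that spawns a random number of apples one at a time.
; Each apple gets a random XY offset from the tree, a fixed world height and random rotation.
; BeginPlay randomizes SpawnSpeed, which this graph never reads.
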(event `self.ReceiveBeginPlay`
  (set `self.SpawnSpeed` (`KismetMathLibrary.RandomFloatInRange` 0.5 5.0)))

(event `self.StaticMesh.OnComponentHit`
  (params (HitComponent :type "PrimitiveComponent Object Reference") (OtherActor :type "Actor Object Reference") (OtherComp :type "PrimitiveComponent Object Reference") (NormalImpulse :type "Vector Structure") (Hit :type "HitResult Structure (by ref)"))
  ;[1 1 1] Take only first hit and with basket
  (cast `/Game/ApplePicker/Blueprints/Gameplay/BP_Basket` OtherActor)
  (if (> Hit_Distance 1.0)
    (`self.WhileLoopWithDelay` (`KismetMathLibrary.RandomIntegerInRange` 1 (`self.Max Spawn Apples`)) 0.25
      (:`Loop Body`
        (bind _returnvalue (`self.Get Spawn Apple Transform`))
        (`|SpawnActorFromClass` (`self.SpawnAppleClass`) _returnvalue "AlwaysSpawn" "OverrideRootScale" null null)))))

(fn `Get Spawn Apple Transform`
  (returns (ReturnValue :type "Transform Structure"))
  (bind _returnvalue (`self.GetTransform`))
  (bind _spawnexpensionmin (`self.SpawnExpensionMin`))
  (bind _spawnexpensionmax (`self.SpawnExpensionMax`))
  (return (`KismetMathLibrary.MakeTransform` (`KismetMathLibrary.MakeVector` (+ (.x (.location _returnvalue)) (`KismetMathLibrary.RandomFloatInRange` _spawnexpensionmin _spawnexpensionmax)) (+ (.y (.location _returnvalue)) (`KismetMathLibrary.RandomFloatInRange` _spawnexpensionmin _spawnexpensionmax)) 100.0) (`KismetMathLibrary.RandomRotator` false))))

(fn `UserConstructionScript`)